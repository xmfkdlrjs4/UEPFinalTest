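; HeroBP is a player-controlled hero character with world-axis movement, a mouse-driven point marker and a punch attack.
; BeginPlay spawns a MousePointBP at the hero's location, shows the cursor and adds the UIWB widget to the viewport.
; Forward and right axes drive movement along fixed world X and Y.
; Two separate LeftMouseClicked handlers move the marker to the Visibility trace hit under the cursor and play the punching montage.
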(event `self.ReceiveBeginPlay`
  (bind _returnvalue (`|SpawnActorFromClass` "/Game/UI/MousePointBP.MousePointBP_C" (`KismetMathLibrary.Conv_VectorToTransform` (`self.K2_GetActorLocation`)) "Undefined" "OverrideRootScale"))
  (set `self.MouseClickPoint` _returnvalue)
  (set `PlayerController.bShowMouseCursor` true (`GameplayStatics.GetPlayerController` 0))
  (bind _returnvalue_2 (`|CreateWidget` "/Game/UI/UIWB.UIWB_C"))
  (bind _output_get (set `self.UI` _returnvalue_2))
  (`UserWidget.AddToViewport` _output_get 0))

(event `InputAction|LeftMouseClicked`
  (params (Key :type "Key Structure" :default "AnyKey"))
  (:`Pressed`
    (`self.K2_SetActorLocation` (`self.MouseClickPoint`) (`.Location` (`GameplayStatics.BreakHitResult` (`PlayerController.GetHitResultUnderCursorByChannel` (`GameplayStatics.GetPlayerController` 0) "TraceTypeQuery1" true))) false false)))

(event `InputAxis|forward`
  (params (AxisValue :type "Float (single-precision)"))
  (`self.AddMovementInput` (1.0 0.0 0.0) AxisValue))

(event `/Game/Enemy/DecreaseHP.NewFunction_0`
  (params (HP :type "Float (single-precision)")))

(event `InputAxis|right`
  (params (AxisValue :type "Float (single-precision)"))
  (`self.AddMovementInput` (0.0 1.0 0.0) AxisValue))

(event `InputAction|LeftMouseClicked`
  (params (Key :type "Key Structure" :default "AnyKey"))
  (:`Pressed`
    (`self.PlayAnimMontage` "/Game/StarterContent/AnimationAssets/UE4_Mannequin/Mesh/PunchingMontage.PunchingMontage")))

(fn `UserConstructionScript`)